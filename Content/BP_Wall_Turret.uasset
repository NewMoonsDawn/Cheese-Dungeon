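; Wall turret with Paper2D flipbook animation that periodically fires projectiles from its BulletSpawnPoint.
; A looping timer with a configurable initial delay calls Shoot, which forwards to the Shooty event so the sequence can use a Delay.
; Shooty pauses the timer, plays the firing flipbook for one second, spawns a projectile with set max speed and lifespan, then resumes.
; The timer period subtracts that second from ShootDelay.
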(event Custom|Shooty
  (bind _bulletspawnpoint (Variables|Default|GetBulletSpawnPoint))
  (bind _paperflipbook (Variables|Default|GetPaperFlipbook))
  (bind _returnvalue (Transformation|GetWorldTransform _bulletspawnpoint))
  (Class|KismetSystemLibrary|PauseTimer 0 "Shoot")
  (Sprite|SetFlipbook _paperflipbook "/Game/Sprites/Frog_Statue_FS/FS.FS")
  (Utilities|FlowControl|Delay 1.0)
  (bind _returnvalue_2 (Game|SpawnActorfromClass "/Game/BP_Wall_Turret_Projectile.BP_Wall_Turret_Projectile_C" (Math|Transform|MakeTransform (.location _returnvalue) (.rotation _returnvalue)) "Undefined" "MultiplyWithRoot" 0 0))
  (Variables|/Script/Engine.ProjectileMovementComponent|SetMaxSpeed (Variables|/Game/BP_Wall_Turret_Projectile.BP_Wall_Turret_Projectile_C|GetProjectileMovement _returnvalue_2) (Variables|Default|GetSpeed))
  (Actor|SetLifeSpan _returnvalue_2 (Variables|Default|GetLifespan))
  (Sprite|SetFlipbook _paperflipbook "/Game/Sprites/Frog_Statue_FS/Sprites/FSIdle.FSIdle")
  (Class|KismetSystemLibrary|UnPauseTimer 0 "Shoot"))

(event EventBeginPlay
  (Utilities|Time|SetTimerbyFunctionName 0 "Shoot" (- (Variables|Default|GetShootDelay) 1.0) true (Variables|Default|GetInitialDelay)))

(event EventTick
  (params (DeltaSeconds :type Float%20%28single-precision%29)))

(fn ConstructionScript)

(fn Shoot
  (CallFunction|Shooty))