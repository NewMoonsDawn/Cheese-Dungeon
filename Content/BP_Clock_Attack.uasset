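; Clock hazard actor with rotating arms that damages BP_ThirdPersonCharacter on contact.
; After a start delay, looping timers step the big arm, and the small arm if TwoArmed, in yaw by configurable amount, direction and interval.
; Without TwoArmed, the small arm is hidden and Box1 overlaps are disabled, both only once the delay ends.
; Four box triggers each apply damage on begin overlap.
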(event OnComponentBeginOverlap(Box)
  (params (OverlappedComponent :type Primitive%20Component%20Object%20Reference) (OtherActor :type Actor%20Object%20Reference) (OtherComp :type Primitive%20Component%20Object%20Reference) (OtherBodyIndex :type Integer) (bFromSweep :type Boolean) (SweepResult :type Hit%20Result%20Structure%20%28by%20ref%29))
  (bind _asbp_third_person_character (Utilities|Casting|CastToBP_ThirdPersonCharacter OtherActor))
  (Game|Damage|ApplyDamage _asbp_third_person_character 1.0 0 0))

(event OnComponentBeginOverlap(Box1)
  (params (OverlappedComponent :type Primitive%20Component%20Object%20Reference) (OtherActor :type Actor%20Object%20Reference) (OtherComp :type Primitive%20Component%20Object%20Reference) (OtherBodyIndex :type Integer) (bFromSweep :type Boolean) (SweepResult :type Hit%20Result%20Structure%20%28by%20ref%29))
  (bind _asbp_third_person_character (Utilities|Casting|CastToBP_ThirdPersonCharacter OtherActor))
  (Game|Damage|ApplyDamage _asbp_third_person_character 1.0 0 0))

(event OnComponentBeginOverlap(Box2)
  (params (OverlappedComponent :type Primitive%20Component%20Object%20Reference) (OtherActor :type Actor%20Object%20Reference) (OtherComp :type Primitive%20Component%20Object%20Reference) (OtherBodyIndex :type Integer) (bFromSweep :type Boolean) (SweepResult :type Hit%20Result%20Structure%20%28by%20ref%29))
  (bind _asbp_third_person_character (Utilities|Casting|CastToBP_ThirdPersonCharacter OtherActor))
  (Game|Damage|ApplyDamage _asbp_third_person_character 1.0 0 0))

(event OnComponentBeginOverlap(Box3)
  (params (OverlappedComponent :type Primitive%20Component%20Object%20Reference) (OtherActor :type Actor%20Object%20Reference) (OtherComp :type Primitive%20Component%20Object%20Reference) (OtherBodyIndex :type Integer) (bFromSweep :type Boolean) (SweepResult :type Hit%20Result%20Structure%20%28by%20ref%29))
  (bind _asbp_third_person_character (Utilities|Casting|CastToBP_ThirdPersonCharacter OtherActor))
  (Game|Damage|ApplyDamage _asbp_third_person_character 1.0 0 0))

(event Custom|SpinBigArm
  (bind _clockarmbig (Variables|Default|GetClockArmBig))
  (bind _returnvalue (Transformation|GetWorldRotation _clockarmbig))
  (Transformation|SetWorldRotation _clockarmbig (Math|Rotator|MakeRotator (.roll _returnvalue) (.pitch _returnvalue) (+ (.yaw _returnvalue) (* (Variables|Default|GetBigArmSpinAmount) (Variables|Default|GetClockwiseBig)))) false false))

(event Custom|SpinSmallArm
  (bind _clockarmsmall (Variables|Default|GetClockArmSmall))
  (bind _returnvalue (Transformation|GetWorldRotation _clockarmsmall))
  (Transformation|SetWorldRotation _clockarmsmall (Math|Rotator|MakeRotator (.roll _returnvalue) (.pitch _returnvalue) (+ (.yaw _returnvalue) (* (Variables|Default|GetSmallSpinAmount) (Variables|Default|GetClockwiseSmall)))) false false))

(event EventBeginPlay
  (Utilities|FlowControl|Delay (Variables|Default|GetStartDelay))
  (if (Variables|Default|GetTwoArmed)
    (Utilities|Time|SetTimerbyEvent (delegate Custom|SpinSmallArm) (Variables|Default|GetDelayBetweenTicksSmall) true)
    (else
      (Variables|/Script/Engine.PrimitiveComponent|SetbGenerateOverlapEvents (Variables|Default|GetBox1) false)
      (Rendering|SetVisibility (Variables|Default|GetClockArmSmall) false true)))
  (Utilities|Time|SetTimerbyEvent (delegate Custom|SpinBigArm) (Variables|Default|GetDelayBetweenTicksBig) true))

(fn ConstructionScript)