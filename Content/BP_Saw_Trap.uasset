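; Saw trap that moves its Sphere with timelines and damages the third-person character on Box overlap, then pauses overlaps for a cooldown.
; It starts at the last "Position"-tagged component, then after a delay loops through those points if both distances are zero.
; Otherwise it shuttles by X/Y distance, flipping sign each run.
; Both modes lerp from the Sphere's current location each update, with sweep.
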(event OnComponentBeginOverlap(Box)
  (params (OverlappedComponent :type Primitive%20Component%20Object%20Reference) (OtherActor :type Actor%20Object%20Reference) (OtherComp :type Primitive%20Component%20Object%20Reference) (OtherBodyIndex :type Integer) (bFromSweep :type Boolean) (SweepResult :type Hit%20Result%20Structure%20%28by%20ref%29))
  (bind _box (Variables|Default|GetBox))
  (bind _asbp_third_person_character (Utilities|Casting|CastToBP_ThirdPersonCharacter OtherActor))
  (Variables|/Script/Engine.PrimitiveComponent|SetbGenerateOverlapEvents _box false)
  (Game|Damage|ApplyDamage _asbp_third_person_character 1.0 0 0)
  (Utilities|FlowControl|Delay 5.0)
  (Variables|/Script/Engine.PrimitiveComponent|SetbGenerateOverlapEvents _box true))

(event Custom|Zoom
  (bind _sphere (Variables|Default|GetSphere))
  (bind _returnvalue (Transformation|GetWorldLocation _sphere))
  (Components|Timeline|SetPlayRate (Variables|Default|GetTimeline) (Variables|Default|GetSpeed))
  (bind _newtrack_0 (Timeline|Timeline PlayFromStart)
    (:Update
      (Transformation|SetWorldLocation (Variables|Default|GetSphere) (Math|Vector|Lerp(Vector) (Transformation|GetWorldLocation (Variables|Default|GetSphere)) (Math|Vector|MakeVector (+ (.x _returnvalue) (Variables|Default|GetDistanceX)) (+ (.y _returnvalue) (Variables|Default|GetDistanceY)) (.z _returnvalue)) _newtrack_0) true false))
    (:Finished
      (Utilities|FlowControl|Delay (Variables|Default|GetDelayBetweenMovement))
      (Variables|Default|SetDistanceX (* (Variables|Default|GetDistanceX) -1.0))
      (Variables|Default|SetDistanceY (* (Variables|Default|GetDistanceY) -1.0))
      (CallFunction|Zoom))))

(event Custom|Go%20To%20Point
  (bind _sphere (Variables|Default|GetSphere))
  (Components|Timeline|SetPlayRate (Variables|Default|GetTimeline_0) (Variables|Default|GetSpeed))
  (bind _newtrack_0 (Timeline|Timeline_0 PlayFromStart)
    (:Update
      (Transformation|SetWorldLocation _sphere (Math|Vector|Lerp(Vector) (Transformation|GetWorldLocation _sphere) (Transformation|GetWorldLocation (Utilities|Array|Get(acopy) (Variables|Default|GetPositions) (Variables|Default|GetPostionIndex))) _newtrack_0) true false))
    (:Finished
      (bind _result (Math|Integer|IncrementInt (Variables|Default|GetPostionIndex))
        (:%20%20
          (if (>= _result (Utilities|Array|Length (Variables|Default|GetPositions)))
            (Variables|Default|SetPostionIndex 0))
          (Utilities|FlowControl|Delay (Variables|Default|GetDelayBetweenMovement))
          (CallFunction|GotoPoint))))))

(event EventBeginPlay
  (Utilities|FlowControl|Delay 0.1)
  (bind _output_get (Variables|Default|SetPositions (Actor|GetComponentsbyTag "/Script/Engine.SceneComponent" "Position")))
  (Transformation|SetWorldLocation (Variables|Default|GetSphere) (Transformation|GetWorldLocation (Utilities|Array|Get(acopy) _output_get (Utilities|Array|LastIndex _output_get))) false false)
  (Utilities|FlowControl|Delay (Variables|Default|GetDelayBeforeStart))
  (if (and (== (Variables|Default|GetDistanceX) 0.0) (== (Variables|Default|GetDistanceY) 0.0))
    (CallFunction|GotoPoint)
    (else
      (CallFunction|Zoom)))
  (Development|PrintString "In Event"))

(fn ConstructionScript)