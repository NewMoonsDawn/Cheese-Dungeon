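; Drop-off station where the third-person player character deposits carried cheese on overlap.
; On BeginPlay it gathers its Cheese-tagged Paper2D flipbook components to serve as deposit slots.
; Each deposit switches the next slots to the CB flipbook, advances the running Cheese count and calls CheeseDeposited on the character.
; A separate flipbook shows unless the player is out of time, then hides after a short delay.
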(event EventBeginPlay
  (Variables|Default|SetFlipbooks (Actor|GetComponentsbyTag "/Script/Paper2D.PaperFlipbookComponent" "Cheese")))

(event Collision|EventActorBeginOverlap
  (params (OtherActor :type Actor%20Object%20Reference))
  (bind _asbp_third_person_character (Utilities|Casting|CastToBP_ThirdPersonCharacter OtherActor))
  (if (Variables|/Game/ThirdPerson/Blueprints/BP_ThirdPersonCharacter.BP_ThirdPersonCharacter_C|GetHoldingCheese _asbp_third_person_character)
    (Utilities|FlowControl|Sequence
      (:then_0
        (if (not (Variables|/Game/ThirdPerson/Blueprints/BP_ThirdPersonCharacter.BP_ThirdPersonCharacter_C|GetOutOfTime _asbp_third_person_character))
          (Rendering|SetVisibility (Variables|Default|GetPaperFlipbook7) true false)))
      (:then_1
        (for _index (range (Variables|Default|GetCheese) (- (+ (Variables|Default|GetCheese) (Variables|/Game/ThirdPerson/Blueprints/BP_ThirdPersonCharacter.BP_ThirdPersonCharacter_C|GetCheeseHeld _asbp_third_person_character)) 1))
          (Sprite|SetFlipbook (Utilities|Array|Get(acopy) (Variables|Default|GetFlipbooks) _index) "/Game/Sprites/Cheese_C/CB.CB"))
        (Variables|Default|SetCheese (+ (Variables|Default|GetCheese) (Variables|/Game/ThirdPerson/Blueprints/BP_ThirdPersonCharacter.BP_ThirdPersonCharacter_C|GetCheeseHeld _asbp_third_person_character)))
        (Default|CheeseDeposited _asbp_third_person_character)
        (Utilities|FlowControl|Delay 3.0)
        (Rendering|SetVisibility (Variables|Default|GetPaperFlipbook7) false false)))))

(fn ConstructionScript)