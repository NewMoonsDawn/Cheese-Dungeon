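; Spike trap actor that damages and shrinks the player, firing on a looping timer or when stepped on.
; Trigger pauses the timer and plays staged Paper2D flipbooks through delays, flagging damage only during one stage.
; A fast looping timer polls that flag while the player overlaps the Box, then disables Box overlap events for a cooldown after a hit.
; Timeline-driven spike movement remains but never runs.
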(event OnComponentBeginOverlap(Box)
  (params (OverlappedComponent :type Primitive%20Component%20Object%20Reference) (OtherActor :type Actor%20Object%20Reference) (OtherComp :type Primitive%20Component%20Object%20Reference) (OtherBodyIndex :type Integer) (bFromSweep :type Boolean) (SweepResult :type Hit%20Result%20Structure%20%28by%20ref%29))
  (Utilities|Casting|CastToBP_ThirdPersonCharacter OtherActor)
  (Utilities|Time|SetTimerbyFunctionName 0 "CheckDamage" 0.001 true))

(event OnComponentBeginOverlap(PlayerStepDetector)
  (params (OverlappedComponent :type Primitive%20Component%20Object%20Reference) (OtherActor :type Actor%20Object%20Reference) (OtherComp :type Primitive%20Component%20Object%20Reference) (OtherBodyIndex :type Integer) (bFromSweep :type Boolean) (SweepResult :type Hit%20Result%20Structure%20%28by%20ref%29))
  (Utilities|Casting|CastToBP_ThirdPersonCharacter OtherActor)
  (if (Variables|Default|GetActivateOnPlayerStep)
    (if (> (.x (Transformation|GetActorScale3D)) 1.0)
      (Utilities|FlowControl|Delay 0.5))
    (CallFunction|Trigger)))

(event OnComponentEndOverlap(Box)
  (params (OverlappedComponent :type Primitive%20Component%20Object%20Reference) (OtherActor :type Actor%20Object%20Reference) (OtherComp :type Primitive%20Component%20Object%20Reference) (OtherBodyIndex :type Integer))
  (Utilities|Casting|CastToBP_ThirdPersonCharacter OtherActor)
  (Utilities|Time|ClearTimerbyFunctionName 0 "CheckDamage"))

(event Custom|Trigger
  (bind _paperflipbook (Variables|Default|GetPaperFlipbook))
  (Class|KismetSystemLibrary|PauseTimer 0 "Spike")
  (Sprite|SetFlipbook _paperflipbook "/Game/Sprites/Trap_Mouth_TM/TMStage2.TMStage2")
  (Utilities|FlowControl|Delay 1.0)
  (Sprite|SetFlipbook _paperflipbook "/Game/Sprites/Trap_Mouth_TM/TMStage3.TMStage3")
  (Utilities|FlowControl|Delay 1.0)
  (Variables|Default|SetDoingDamage true)
  (Sprite|SetFlipbook _paperflipbook "/Game/Sprites/Trap_Mouth_TM/TMStage4.TMStage4")
  (Utilities|FlowControl|Delay 0.75)
  (Variables|Default|SetDoingDamage false)
  (Sprite|SetFlipbook _paperflipbook "/Game/Sprites/Trap_Mouth_TM/TMStage5.TMStage5")
  (Utilities|FlowControl|Delay 0.66)
  (Sprite|SetFlipbook _paperflipbook "/Game/Sprites/Trap_Mouth_TM/TMStage1.TMStage1")
  (Class|KismetSystemLibrary|UnPauseTimer 0 "Spike"))

(event Custom|TurnOverlaptEventson
  (Utilities|FlowControl|Delay 5.0)
  (Variables|/Script/Engine.PrimitiveComponent|SetbGenerateOverlapEvents (Variables|Default|GetBox) true))

(event EventBeginPlay
  (bind _asbp_third_person_character (Utilities|Casting|CastToBP_ThirdPersonCharacter (Game|GetPlayerCharacter 0)))
  (Variables|Default|SetAs%20BP%20Third%20Person%20Character _asbp_third_person_character)
  (if (not (Variables|Default|GetActivateOnPlayerStep))
    (Utilities|Time|SetTimerbyFunctionName 0 "Spike" (- (Variables|Default|GetDelay) 1.25) true (Variables|Default|GetInitialDelay))))

(fn ConstructionScript)

(fn Spike
  (CallFunction|Trigger))

(fn CheckDamage
  (if (Variables|Default|GetDoingDamage)
    (Utilities|Time|ClearTimerbyFunctionName 0 "CheckDamage")
    (Variables|/Script/Engine.PrimitiveComponent|SetbGenerateOverlapEvents (Variables|Default|GetBox) false)
    (Game|Damage|ApplyDamage (Variables|Default|GetAs%20BP%20Third%20Person%20Character) 1.0 0 0)
    (Default|Shrink (Variables|Default|GetAs%20BP%20Third%20Person%20Character))
    (CallFunction|TurnOverlaptEventson)))